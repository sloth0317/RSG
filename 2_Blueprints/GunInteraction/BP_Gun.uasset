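; BP_Gun is a gun that the player can interact with to pick up and later drop, apparently serving as a base for specific weapons.
; A GunState switch toggles physics and collision on the box and skeletal mesh between Dropped, the starting state, and Equipped.
; Interaction shows a "Pick Up" prompt attached to the mesh, calls PickUpGun on the player and equips the gun.
; Damage, interval and automatic-fire getters return placeholder defaults.
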(event EventBeginPlay
  (Public|SetGunState "NewEnumerator0" (Variables|Default|GetBox) (Variables|Default|GetSkeletalMesh)))

(event EventOnInteracted
  (params (Player :type First%20Person%20Character%20Object%20Reference))
  (Default|PickUpGun Player self)
  (Public|SetGunState "NewEnumerator1" (Variables|Default|GetBox) (Variables|Default|GetSkeletalMesh)))

(fn ConstructionScript
  (|CallParentFunction))

(fn GetInteractionText
  (return "Pick Up"))

(fn GetInteractionTextAttach
  (return (Variables|Default|GetSkeletalMesh)))

(fn SetGunState
  (params (NewGunState :type EGunState%20Enum :default "NewEnumerator0") (BoxCollision :type Box%20Component%20Object%20Reference) (SkeletalMesh :type Skeletal%20Mesh%20Component%20Object%20Reference))
  (bind _output_get (Variables|Private|SetGunState NewGunState))
  (switch Utilities|FlowControl|Switch|SwitchonEGunState _output_get
    (:NewEnumerator0
      (Collision|SetCollisionProfileName BoxCollision "OverlapAllDynamic" true :!class /Script/Engine.PrimitiveComponent)
      (Collision|SetCollisionResponsetoChannel BoxCollision "ECC_GameTraceChannel1" "ECR_Ignore")
      (Physics|SetSimulatePhysics SkeletalMesh true)
      (Collision|SetCollisionProfileName SkeletalMesh "DroppedGun" true :!class /Script/Engine.PrimitiveComponent))
    (:NewEnumerator1
      (Collision|SetCollisionProfileName BoxCollision "NoCollision" true :!class /Script/Engine.PrimitiveComponent)
      (Physics|SetSimulatePhysics SkeletalMesh false)
      (Collision|SetCollisionProfileName SkeletalMesh "NoCollision" true :!class /Script/Engine.PrimitiveComponent)
      (Transformation|ResetRelativeTransform SkeletalMesh))))

(fn Drop
  (params (BoxCollision :type Box%20Component%20Object%20Reference) (SkeletalMesh :type Skeletal%20Mesh%20Component%20Object%20Reference))
  (Public|SetGunState "NewEnumerator0" BoxCollision SkeletalMesh))

(fn GetGunDamage
  (return 0.0))

(fn GetGunInterval
  (return 0.0))

(fn GetIsGunAuto
  (return false))