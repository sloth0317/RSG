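; Target dummy NPC that plays a looping rifle idle and can be dismembered by bullet hits.
; Bullet damage lowers per-body-part HP keyed by physical material; a depleted part breaks its mapped bone constraint and receives an impulse at the hit bone.
; Breaking spine_01 marks it dead, enabling ragdoll physics and disabling capsule collision, then a timer respawns a fresh copy at the starting transform.
; Restore-gun logic for broken bones is present but never runs.
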(event EventBeginPlay
  (Variables|Dismemberment|SetBodyPartsHP (Variables|Dismemberment|GetBodyPartsMaxHP))
  (Components|Animation|PlayAnimation (Variables|Character|GetMesh) "/Game/1_Marketplace/AnimStarterPack/Idle_Rifle_Ironsights.Idle_Rifle_Ironsights" true)
  (Variables|Default|SetRespawnTransform (Transformation|GetActorTransform)))

(event EventHittedbyBullet
  (params (Damage :type Float%20%28single-precision%29) (HittedPhysMat :type Physical%20Material%20Object%20Reference) (HitBoneName :type Name :default "None") (EventInstigator :type Controller%20Object%20Reference) (DamageCauser :type Actor%20Object%20Reference))
  (Dismemberment|AnyDamage Damage HittedPhysMat HitBoneName)
  (if (Variables|Default|GetIsDead)
    (Utilities|FlowControl|DoOnce false
      (:Completed
        (Collision|SetCollisionEnabled (Variables|Collision|GetCapsuleComponent) "NoCollision")
        (Audio|Components|Audio|Stop (Variables|Character|GetMesh))
        (Utilities|Time|SetTimerbyFunctionName 0 "Respawn" 3.0)))))

(fn ConstructionScript)

(fn AnyDamage
  (params (Damage :type Float%20%28single-precision%29) (HittedPhysMat :type Physical%20Material%20Object%20Reference) (HitBoneName :type Name))
  (Variables|Dismemberment|SetAppliedDamage Damage)
  (Variables|Dismemberment|SetHitted%20Phys%20Mat HittedPhysMat)
  (Variables|Dismemberment|SetHitBoneName HitBoneName)
  (bind _bodypartsbroke (Dismemberment|ApplyDamagetoPhysMat))
  (if _bodypartsbroke
    (Dismemberment|Dismemberment)
    (Dismemberment|ApplyPhysics)))

(fn ApplyDamagetoPhysMat
  (bind _hitted_phys_mat (Variables|Dismemberment|GetHitted%20Phys%20Mat))
  (bind _bodypartshp (Variables|Dismemberment|GetBodyPartsHP))
  (bind (_value _returnvalue) (Utilities|Map|Find _bodypartshp _hitted_phys_mat))
  (if _returnvalue
    (Utilities|Map|Add _bodypartshp _hitted_phys_mat (Math|Float|Max(Float) (- _value (Variables|Dismemberment|GetAppliedDamage)) 0.0))
    (return (<= (.Value (Utilities|Map|Find _bodypartshp _hitted_phys_mat)) 0.0))))

(fn Dismemberment
  (bind _hitted_phys_mat (Variables|Dismemberment|GetHitted%20Phys%20Mat))
  (bind _physmattobone (Variables|Dismemberment|GetPhysMatToBone))
  (bind (_value _returnvalue) (Utilities|Map|Find _physmattobone _hitted_phys_mat))
  (bind _returnvalue_2 (Utilities|Name|Equal(Name) _value "spine_01"))
  (if _returnvalue
    (Class|SkeletalMeshComponent|BreakConstraint (Variables|Character|GetMesh) (Utilities|CalculateImpulse) (Utilities|GetSocketLocation) _value)
    (if _returnvalue_2
      (Variables|Default|SetIsDead _returnvalue_2)
      (Utilities|Array|Add (Variables|Dismemberment|GetBrokenBones) _value))))

(fn ApplyPhysics
  (bind _mesh (Variables|Character|GetMesh))
  (bind _bodypartshp (Variables|Dismemberment|GetBodyPartsHP))
  (if (Variables|Default|GetIsDead)
    (Utilities|Map|Add _bodypartshp "/Game/4_Meshes/BPD_Physics/PhysMat_Head.PhysMat_Head" 0.0)
    (Utilities|Map|Add _bodypartshp "/Game/4_Meshes/BPD_Physics/PhysMat_Body.PhysMat_Body" 0.0)
    (Physics|SetSimulatePhysics _mesh true) ; 스위치 부위가 파괴되면 물리 적용
  )
  (Physics|AddImpulseatLocation _mesh (Utilities|CalculateImpulse) (Utilities|GetSocketLocation) (Variables|Dismemberment|GetHitBoneName)) ; 파괴되서 떨어진 부위에 충격을 가함
)

(fn Respawn
  (Actor|DestroyActor)
  (Game|SpawnActorfromClass (Utilities|GetClass self) (Variables|Default|GetRespawnTransform) "AlwaysSpawn" 0 0))