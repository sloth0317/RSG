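; AI controller for the enemy boss that starts the EnemyBoss behavior tree on BeginPlay.
; Tick only calls its parent, so the controller adds no per-frame logic.
; An unconnected branch would write the IsDefenceStatus blackboard enum from a Player tag check and distance thresholds, but it never runs.
; That branch uses SetDefenceActionStatus, a helper that simply returns the enum value passed in.
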(event EventBeginPlay
  (|CallParentFunction)
  (AI|RunBehaviorTree "/Game/2_Blueprints/AIControl/EnemyBoss.EnemyBoss"))

(event EventTick
  (params (DeltaSeconds :type Float%20%28single-precision%29))
  (|CallParentFunction DeltaSeconds))

(fn ConstructionScript
  (|CallParentFunction))

(fn SetDefenceActionStatus
  (params (DefenceStatus :type DefenceState%20Enum :default "NewEnumerator0"))
  (return DefenceStatus))